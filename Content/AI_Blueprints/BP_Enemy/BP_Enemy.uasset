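; BP_Enemy is a basic enemy actor with a Health value that can take damage and die.
; Its TakeDMG event subtracts the given amount from Health, then destroys the actor when CheckIfDead finds Health at or below zero.
; Debug strings print on BeginPlay and on each hit, and the graphs contain no movement or attack logic.
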(event Custom|Take%20DMG
  (params (By%20Amount :type Float%20%28double-precision%29))
  (Development|PrintString "Owie :[" true true "(R=0.000000,G=0.660000,B=1.000000,A=1.000000)" 5.0)
  (Variables|Default|SetHealth (- (Variables|Default|GetHealth) By%20Amount))
  (if (CallFunction|CheckifDead (Variables|Default|GetHealth))
    (Actor|DestroyActor)))

(event EventBeginPlay
  (Development|PrintString "I will now murder you :]" true true "(R=0.000000,G=0.660000,B=1.000000,A=1.000000)" 1e+01))

(event Collision|EventActorBeginOverlap
  (params (OtherActor :type Actor%20Object%20Reference)))

(event EventTick
  (params (DeltaSeconds :type Float%20%28single-precision%29)))

(fn ConstructionScript)

(fn CheckifDead
  (params (Health :type Float%20%28double-precision%29))
  (return (<= Health 0.0)))