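; Test actor that repeatedly damages every BP_Enemy in the level to exercise enemy damage handling.
; BeginPlay enters the same chain as the GiveDMG event, which gathers all BP_Enemy actors and calls TakeDMG on each with a small random amount.
; Debug strings print the enemy count and hit progress, then a short Delay calls GiveDMG again, forming an endless loop without Tick.
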(event Custom|GiveDMG
  (bind _outactors (Actor|GetAllActorsOfClass "/Game/AI_Blueprints/BP_Enemy/BP_Enemy.BP_Enemy_C")) ; Find all of the BP_Enemies
  (Development|PrintString (Utilities|String|Append "There are " (Utilities|String|ToString(Integer) (Utilities|Array|Length _outactors)) " enemies in the level.") true true "(R=0.000000,G=0.660000,B=1.000000,A=1.000000)" 2e+01)
  (for _array_element _outactors
    (Default|TakeDMG _array_element (Math|Random|RandomFloatinRange 0.1 0.5))
    (Development|PrintString "We dead" true true "(R=0.000000,G=0.660000,B=1.000000,A=1.000000)" 5.0))
  (Development|PrintString "We did damaged" true true "(R=0.000000,G=0.660000,B=1.000000,A=1.000000)" 1e+01)
  (Utilities|FlowControl|Delay 2.0)
  (CallFunction|GiveDMG))

(event EventBeginPlay
  (bind _outactors (Actor|GetAllActorsOfClass "/Game/AI_Blueprints/BP_Enemy/BP_Enemy.BP_Enemy_C")) ; Find all of the BP_Enemies
  (Development|PrintString (Utilities|String|Append "There are " (Utilities|String|ToString(Integer) (Utilities|Array|Length _outactors)) " enemies in the level.") true true "(R=0.000000,G=0.660000,B=1.000000,A=1.000000)" 2e+01)
  (for _array_element _outactors
    (Default|TakeDMG _array_element (Math|Random|RandomFloatinRange 0.1 0.5))
    (Development|PrintString "We dead" true true "(R=0.000000,G=0.660000,B=1.000000,A=1.000000)" 5.0))
  (Development|PrintString "We did damaged" true true "(R=0.000000,G=0.660000,B=1.000000,A=1.000000)" 1e+01)
  (Utilities|FlowControl|Delay 2.0)
  (CallFunction|GiveDMG))

(event Collision|EventActorBeginOverlap
  (params (OtherActor :type Actor%20Object%20Reference)))

(event EventTick
  (params (DeltaSeconds :type Float%20%28single-precision%29)))

(fn ConstructionScript)