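; BP_Item is an item actor that can be picked up, thrown and given a primary action.
; PickUp disables Cube collision, sets physics simulation on and attaches to the hand_r socket of the passed component.
; Drop restores physics-only collision, detaches Cube and the passed skeletal mesh, then applies a fixed forward-and-up force as acceleration.
; PrimaryAction is a stub that only prints debug text.
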(event Custom|PickUp
  (params (Capsule%20Component :type Scene%20Component%20Object%20Reference))
  ;[1 1 1] Pick up item
  (Development|PrintString "PickUp" true true "(R=1.000000,G=0.000000,B=0.076571,A=1.000000)" 5.0)
  (Collision|SetCollisionEnabled (Variables|Default|GetCube) "NoCollision")
  (Physics|SetSimulatePhysics (Variables|Default|GetCube) true)
  (Transformation|AttachComponentToComponent Capsule%20Component "hand_r" "SnapToTarget" "SnapToTarget" "KeepRelative" true))

(event Custom|Drop
  (params (Skeletal%20Mesh :type Scene%20Component%20Object%20Reference))
  ;[1 1 1] Throws item
  (Development|PrintString "Drop" true true "(R=0.296141,G=1.000000,B=0.000000,A=1.000000)" 5.0)
  (Collision|SetCollisionEnabled (Variables|Default|GetCube) "PhysicsOnly")
  (Transformation|DetachFromComponent (Variables|Default|GetCube) "KeepWorld" "KeepWorld" "KeepWorld" true)
  (Physics|SetSimulatePhysics (Variables|Default|GetCube) true)
  (Physics|AddForce (Variables|Default|GetCube) "500.000000,0.000000,250.000000" "None" true))

(event Custom|Primary%20Action
  (Development|PrintString "Primary Action" true true "(R=0.000000,G=0.660000,B=1.000000,A=1.000000)" 5.0))

(fn ConstructionScript)